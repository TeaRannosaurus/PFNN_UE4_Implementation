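; BP_TestCharacter is a test character that automatically cycles the player's view through its own camera components.
; BeginPlay gathers the cameras, and a Tick timer calls NextCamera at a set interval to activate only the next one, wrapping around.
; Each switch sets the player's view target to the character with a cubic blend.
; A separate MovetoWaypoint event, not called here, sends it by AI move to the current waypoint.
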(event EventBeginPlay
  (CallFunction|SetCameras))

(event EventTick
  (params (DeltaSeconds :type Float%20%28single-precision%29))
  (CallFunction|UpdateCamera DeltaSeconds))

(event EventMovetoWaypoint
  ;[1 1 1] MovetoWaypoint
  (AI|AIMoveTo self (.location (Utilities|Array|Get(acopy) (Variables|Default|GetWaypoints) (Variables|Default|GetCurrentIndex))) 0 5.0 false))

(fn ConstructionScript)

(fn UpdateCamera
  (params (DeltaTime :type Float%20%28single-precision%29))
  (Variables|Camera|SetTimeSinceLastSwitch (+ (Variables|Camera|GetTimeSinceLastSwitch) DeltaTime))
  (if (>= (Variables|Camera|GetTimeSinceLastSwitch) (Variables|Camera|GetSecondsBetweenSwitches))
    (CallFunction|NextCamera)
    (Variables|Camera|SetTimeSinceLastSwitch 0.0)))

(fn SetCameras
  (Utilities|Array|Clear (Variables|Camera|GetCameras))
  (Variables|Camera|SetCameras (Actor|GetComponentsByClass self "/Script/Engine.CameraComponent")))

(fn NextCamera
  (bind _result (Math|Integer|IncrementInt (Variables|Camera|GetCameraIndex))
    (:%20%20
      (if (>= _result (Utilities|Array|Length (Variables|Camera|GetCameras)))
        (Variables|Camera|SetCameraIndex 0))
      (for (_array_element _array_index) (Variables|Camera|GetCameras)
        (Components|Activation|SetActive _array_element (== (Variables|Camera|GetCameraIndex) _array_index) false))
      (Game|Player|SetViewTargetwithBlend (Game|GetPlayerController 0) self 2.0 "VTBlend_Cubic" 0.0 false))))